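; BP_Player is the player Blueprint that relays lifecycle events to BP_GameMode for UI and saving.
; BeginPlay, PauseGame and OnDeathEvent each cast the game mode, then have it draw the HUD, pause menu or game-over screen respectively.
; On death it first saves the game through the game mode, passing a hardcoded player name and the Age variable as the score.
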(event `self.ReceiveBeginPlay`
  (bind _asbp_game_mode (cast `/Game/Dynamic/GameMode/BP_GameMode` (`GameplayStatics.GetGameMode`)))
  (`/Game/Dynamic/GameMode/BP_GameMode.Draw HUD` _asbp_game_mode))

(event `self.PauseGame`
  (bind _asbp_game_mode (cast `/Game/Dynamic/GameMode/BP_GameMode` (`GameplayStatics.GetGameMode`)))
  (`/Game/Dynamic/GameMode/BP_GameMode.Draw Pause Menu` _asbp_game_mode))

(event `self.OnDeathEvent`
  (bind _asbp_game_mode (cast `/Game/Dynamic/GameMode/BP_GameMode` (`GameplayStatics.GetGameMode`)))
  (`PGameMode.SaveGame` _asbp_game_mode "Ishrak" (`self.Age`))
  (`/Game/Dynamic/GameMode/BP_GameMode.Draw Game Over` _asbp_game_mode))

(fn `UserConstructionScript`)